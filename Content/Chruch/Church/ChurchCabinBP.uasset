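; Church cabin actor with an interactable door and a trigger volume that tracks whether the player is inside.
; Interacting with Box4 plays or reverses a timeline that sets the door's yaw, with IsDoorOpen updated after a short delay.
; Box overlap events set or clear IsCharCabin on the FirstPersonCharacter cached at BeginPlay.
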(event OnComponentBeginOverlap(Box)
  (params (OverlappedComponent :type Primitive%20Component%20Object%20Reference) (OtherActor :type Actor%20Object%20Reference) (OtherComp :type Primitive%20Component%20Object%20Reference) (OtherBodyIndex :type Integer) (bFromSweep :type Boolean) (SweepResult :type Hit%20Result%20Structure%20%28by%20ref%29))
  (bind _as_first_person_character (Variables|Default|GetAs%20First%20Person%20Character))
  (if (== OtherActor _as_first_person_character)
    (Variables|/Game/FirstPersonBP/Blueprints/FirstPersonCharacter.FirstPersonCharacter_C|SetisCharCabin _as_first_person_character true)))

(event OnComponentEndOverlap(Box)
  (params (OverlappedComponent :type Primitive%20Component%20Object%20Reference) (OtherActor :type Actor%20Object%20Reference) (OtherComp :type Primitive%20Component%20Object%20Reference) (OtherBodyIndex :type Integer))
  (bind _as_first_person_character (Variables|Default|GetAs%20First%20Person%20Character))
  (if (== OtherActor _as_first_person_character)
    (Variables|/Game/FirstPersonBP/Blueprints/FirstPersonCharacter.FirstPersonCharacter_C|SetisCharCabin _as_first_person_character false)))

(event EventBeginPlay
  (bind _asfirst_person_character (Utilities|Casting|CastToFirstPersonCharacter (Game|GetPlayerCharacter 0)))
  (Variables|Default|SetAs%20First%20Person%20Character _asfirst_person_character))

(event Collision|EventActorBeginOverlap
  (params (OtherActor :type Actor%20Object%20Reference)))

(event EventTick
  (params (DeltaSeconds :type Float%20%28single-precision%29)))

(event EventInteract
  (params (PlayerRef :type First%20Person%20Character%20Object%20Reference) (HitActor :type Hit%20Result%20Structure) (ObjectRef :type Actor%20Object%20Reference))
  (bind _door (Variables|Default|GetDoor))
  (bind _relativerotation (Variables|/Script/Engine.SceneComponent|GetRelativeRotation _door))
  (if (== (.HitComponent (Collision|BreakHitResult HitActor)) (Variables|Default|GetBox4))
    (if (not (Variables|Default|GetisDoorOpen))
      (Utilities|FlowControl|Sequence
        (:then_0
          (bind _newtrack_0 (Timeline|DoorControlTL Play)
            (:Update
              (Transformation|SetRelativeRotation _door (Math|Rotator|MakeRotator (.roll _relativerotation) (.pitch _relativerotation) _newtrack_0) false false))))
        (:then_1
          (Utilities|FlowControl|Delay 0.75)
          (Variables|Default|SetisDoorOpen true)))
      (else
        (Utilities|FlowControl|Sequence
          (:then_0
            (Timeline|DoorControlTL Reverse))
          (:then_1
            (Utilities|FlowControl|Delay 0.75)
            (Variables|Default|SetisDoorOpen false)))))))

(fn ConstructionScript)