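; EnemyChurchBP is an enemy pawn for a church that can walk a scripted route and chase the first-person player.
; ChurchControl chains AI moves through six locations, then destroys the actor.
; PawnSensing sets a sight flag that a retriggerable delay clears shortly after contact stops.
; Each tick, that flag switches walk speed, triggers chasing within range and updates player distance, with debug prints.
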(event OnSeePawn(PawnSensing)
  (params (Pawn :type Pawn%20Object%20Reference))
  (Utilities|FlowControl|Sequence
    (:then_0
      (Variables|Default|SetcanSeeEnemy true))
    (:then_1
      (Utilities|FlowControl|RetriggerableDelay 0.5)
      (Variables|Default|SetcanSeeEnemy false))))

(event Custom|ChaseEnemy
  (bind _distance (Variables|Default|GetDistance))
  (if (and (<= _distance 1.2e+03) (Variables|Default|GetcanSeeEnemy))
    (AI|AIMoveTo self "0, 0, 0" (stale EventBeginPlay _output_get) 5.0 false
      (:then
        (Development|PrintString (Utilities|String|ToString(Float) _distance))))
    (else
      (Development|PrintString "false"))))

(event Custom|SetPlayerDistance
  (bind _output_get (Variables|Default|SetDistance (Math|Vector|Distance(Vector) (Transformation|GetActorLocation self) (Transformation|GetActorLocation (Variables|Default|GetAs%20First%20Person%20Character))))))

(event Custom|ChurchControl
  (bind _self self)
  (AI|AIMoveTo _self (Variables|Default|GetLocation1) 0 5.0 false
    (:OnSuccess
      (AI|AIMoveTo _self (Variables|Default|GetLocation2) 0 5.0 false
        (:OnSuccess
          (AI|AIMoveTo _self (Variables|Default|GetLocation3) 0 5.0 false
            (:OnSuccess
              (AI|AIMoveTo _self (Variables|Default|GetLocation4) 0 5.0 false
                (:OnSuccess
                  (AI|AIMoveTo _self (Variables|Default|GetLocation5) 0 5.0 false
                    (:OnSuccess
                      (AI|AIMoveTo _self (Variables|Default|GetLocation6) 0 5.0 false
                        (:OnSuccess
                          (Actor|DestroyActor))))))))))))))

(event EventBeginPlay
  (bind _asfirst_person_character (Utilities|Casting|CastToFirstPersonCharacter (Game|GetPlayerCharacter 0)))
  (bind _output_get (Variables|Default|SetAs%20First%20Person%20Character _asfirst_person_character)))

(event Collision|EventActorBeginOverlap
  (params (OtherActor :type Actor%20Object%20Reference)))

(event EventTick
  (params (DeltaSeconds :type Float%20%28single-precision%29))
  (bind _charactermovement (Variables|Character|GetCharacterMovement))
  (Utilities|FlowControl|Sequence
    (:then_0
      (if (Variables|Default|GetcanSeeEnemy)
        (Variables|/Script/Engine.CharacterMovementComponent|SetMaxWalkSpeed _charactermovement 7e+02)
        (else
          (Variables|/Script/Engine.CharacterMovementComponent|SetMaxWalkSpeed _charactermovement 4e+02))))
    (:then_1
      (CallFunction|ChaseEnemy))
    (:then_2
      (CallFunction|SetPlayerDistance))))

(fn ConstructionScript)