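; CarTry2BP is a scripted car actor that drives along a fixed path for a timed sequence involving the player.
; On BeginPlay it shows itself, animates its root's world Y with a timeline, and sets IsStop when that finishes.
; In parallel, a 27.25-second delay triggers BlackImageScreen on the FirstPersonCharacter.
; Tick hides the actor while IsCrash is true, a flag this graph never sets.
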(event EventBeginPlay
  (bind _defaultsceneroot (Variables|Default|GetDefaultSceneRoot))
  (bind _returnvalue (Transformation|GetWorldLocation _defaultsceneroot))
  (Utilities|FlowControl|Sequence
    (:then_0
      (bind _asfirst_person_character (Utilities|Casting|CastToFirstPersonCharacter (Game|GetPlayerCharacter 0)))
      (bind _output_get (Variables|Default|SetAs%20First%20Person%20Character _asfirst_person_character))
      (Utilities|FlowControl|Delay 27.25)
      (Default|BlackImageScreen _output_get))
    (:then_1
      (bind _newtrack_0 (Timeline|Timeline_0 Play)
        (:Update
          (Transformation|SetWorldLocation _defaultsceneroot (Math|Vector|MakeVector (.x _returnvalue) _newtrack_0 (.z _returnvalue)) false false))
        (:Finished
          (Variables|Default|SetisStop true))))
    (:then_2
      (Rendering|SetActorHiddenInGame false))))

(event Collision|EventActorBeginOverlap
  (params (OtherActor :type Actor%20Object%20Reference)))

(event EventTick
  (params (DeltaSeconds :type Float%20%28single-precision%29))
  (if (Variables|Default|GetisCrash)
    (Rendering|SetActorHiddenInGame true)))

(fn ConstructionScript)