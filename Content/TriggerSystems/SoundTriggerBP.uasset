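; SoundTriggerBP is a trigger actor that plays scripted scream or laughter sounds at set locations when the player overlaps it.
; Its collision component filters overlapping actors by the PlayerBPI interface, then calls both GirlScream and Laughts in sequence.
; Each event checks EventNumber, so 1 plays a single scream and 2 plays three staggered laughs at separate positions.
; Nothing limits it to one firing.
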(event OnComponentBeginOverlap(CollisionComponent)
  (params (OverlappedComponent :type Primitive%20Component%20Object%20Reference) (OtherActor :type Actor%20Object%20Reference) (OtherComp :type Primitive%20Component%20Object%20Reference) (OtherBodyIndex :type Integer) (bFromSweep :type Boolean) (SweepResult :type Hit%20Result%20Structure%20%28by%20ref%29))
  (if (Utilities|DoesObjectImplementInterface OtherActor "/Game/Blueprints/Interface/PlayerBPI.PlayerBPI_C")
    (Utilities|FlowControl|Sequence
      (:then_0
        (CallFunction|GirlScream))
      (:then_1
        (CallFunction|Laughts)))))

(event Custom|GirlScream
  (if (== (Variables|Default|GetEventNumber) 1)
    (Audio|PlaySoundatLocation "/Game/Audio/GirlScream.GirlScream" (Variables|Default|GetGirlScreamLocation) "0, 0, 0" 1.0 1.0 0.0 0 0 0)))

(event Custom|Laughts
  (if (== (Variables|Default|GetEventNumber) 2)
    (Audio|PlaySoundatLocation "/Game/Audio/Laughts/Laugh1.Laugh1" (Utilities|Array|Get(acopy) (Variables|Default|GetLaughtsLocation)) "0, 0, 0" 1.0 1.0 0.0 0 0 0)
    (Utilities|FlowControl|Delay 0.75)
    (Audio|PlaySoundatLocation "/Game/Audio/Laughts/Laugh2.Laugh2" (Utilities|Array|Get(acopy) (Variables|Default|GetLaughtsLocation) 1) "0, 0, 0" 1.0 1.0 0.0 0 0 0)
    (Utilities|FlowControl|Delay 0.45)
    (Audio|PlaySoundatLocation "/Game/Audio/Laughts/Laugh3.Laugh3" (Utilities|Array|Get(acopy) (Variables|Default|GetLaughtsLocation) 2) "0, 0, 0" 1.0 1.0 0.0 0 0 0)))

(event EventBeginPlay)

(event Collision|EventActorBeginOverlap
  (params (OtherActor :type Actor%20Object%20Reference)))

(event EventTick
  (params (DeltaSeconds :type Float%20%28single-precision%29)))

(fn ConstructionScript)