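; Interactable well actor that brings up an object, which the player can then take.
; The first Interact freezes player movement and mouse input while a timeline rotates a scene component and animates the Cube's height.
; When it finishes, control returns, the trigger Collision is destroyed and the initially non-colliding Cube gains collision.
; A later Interact simply destroys the Cube.
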(event EventBeginPlay
  (Utilities|FlowControl|Sequence
    (:then_0
      (bind _asfirst_person_character (Utilities|Casting|CastToFirstPersonCharacter (Game|GetPlayerCharacter 0)))
      (Variables|Default|SetAs%20First%20Person%20Character _asfirst_person_character))
    (:then_1
      (Collision|SetCollisionEnabled (Variables|Default|GetCube) "NoCollision"))))

(event Collision|EventActorBeginOverlap
  (params (OtherActor :type Actor%20Object%20Reference)))

(event EventTick
  (params (DeltaSeconds :type Float%20%28single-precision%29)))

(event EventInteract
  (params (PlayerRef :type First%20Person%20Character%20Object%20Reference) (HitActor :type Hit%20Result%20Structure) (ObjectRef :type Actor%20Object%20Reference))
  (bind _as_first_person_character (Variables|Default|GetAs%20First%20Person%20Character))
  (bind _cube (Variables|Default|GetCube))
  (bind _relativelocation (Variables|/Script/Engine.SceneComponent|GetRelativeLocation _cube))
  (bind _charactermovement (Variables|/Script/Engine.Character|GetCharacterMovement _as_first_person_character))
  (if (not (Variables|Default|GetisObjectTakeable))
    (Variables|/Game/FirstPersonBP/Blueprints/FirstPersonCharacter.FirstPersonCharacter_C|SetMouseInputUseable (Variables|Default|GetAs%20First%20Person%20Character) false)
    (Components|Activation|SetActive _charactermovement false false)
    (bind (_direction _well _object) (Timeline|Well Play)
      (:Update
        (Transformation|SetWorldRotation (Variables|Default|GetScene2) (Math|Rotator|MakeRotator 0.0 _well 0.0) false false)
        (Transformation|SetRelativeLocation _cube (Math|Vector|MakeVector (.x _relativelocation) (.y _relativelocation) _object) false false))
      (:Finished
        (Collision|SetCollisionEnabled (Variables|Default|GetCube) "QueryAndPhysics")
        (Variables|Default|SetisObjectTakeable true)
        (Components|Activation|SetActive _charactermovement true false)
        (Variables|/Game/FirstPersonBP/Blueprints/FirstPersonCharacter.FirstPersonCharacter_C|SetMouseInputUseable (Variables|Default|GetAs%20First%20Person%20Character) true)
        (Components|DestroyComponent (Variables|Default|GetCollision))))
    (else
      (Components|DestroyComponent (Variables|Default|GetCube)))))

(fn ConstructionScript)