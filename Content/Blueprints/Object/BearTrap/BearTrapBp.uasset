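; Bear trap actor that snaps shut and immobilizes a FirstPersonCharacter entering its box, until it is dismantled.
; Overlap plays a timeline rotating both jaws, sets IsTraped, and disables the victim's movement component after a short delay.
; Interact locks mouse input and shows a Turkish dismantling message during a timed removal, also freezing the user if unsprung.
; Removal then restores controls, frees any stored victim and destroys the trap.
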(event OnComponentBeginOverlap(Box)
  (params (OverlappedComponent :type Primitive%20Component%20Object%20Reference) (OtherActor :type Actor%20Object%20Reference) (OtherComp :type Primitive%20Component%20Object%20Reference) (OtherBodyIndex :type Integer) (bFromSweep :type Boolean) (SweepResult :type Hit%20Result%20Structure%20%28by%20ref%29))
  (bind _asfirst_person_character (Utilities|Casting|CastToFirstPersonCharacter OtherActor))
  (Variables|Default|SetAs%20First%20Person%20Character _asfirst_person_character)
  (bind (_direction _trap_timeline_a _trap_timeline_b) (Timeline|Trap Play)
    (:Update
      (Utilities|FlowControl|Sequence
        (:then_0
          (Transformation|SetRelativeRotation (Variables|Default|GetBearTrapAnims_Jaw_1) (Math|Rotator|MakeRotator 0.0 _trap_timeline_a 0.0) false false))
        (:then_1
          (Transformation|SetRelativeRotation (Variables|Default|GetBearTrapAnims_Jaw_2) (Math|Rotator|MakeRotator 0.0 _trap_timeline_b 0.0) false false))
        (:then_2
          (Utilities|FlowControl|Delay 0.15)
          (Components|Activation|SetActive (Variables|/Script/Engine.Character|GetCharacterMovement (Variables|Default|GetAs%20First%20Person%20Character)) false false))
        (:then_3
          (Variables|Default|SetisTraped true))))))

(event EventBeginPlay)

(event Collision|EventActorBeginOverlap
  (params (OtherActor :type Actor%20Object%20Reference)))

(event EventTick
  (params (DeltaSeconds :type Float%20%28single-precision%29)))

(event EventInteract
  (params (PlayerRef :type First%20Person%20Character%20Object%20Reference) (HitActor :type Hit%20Result%20Structure))
  (bind _charactermovement (Variables|/Script/Engine.Character|GetCharacterMovement PlayerRef))
  (bind _as_first_person_character (Variables|Default|GetAs%20First%20Person%20Character))
  (bind _playerhudw (Variables|/Game/FirstPersonBP/Blueprints/FirstPersonCharacter.FirstPersonCharacter_C|GetPlayerHudW PlayerRef))
  (bind _playerhudw_2 (Variables|/Game/FirstPersonBP/Blueprints/FirstPersonCharacter.FirstPersonCharacter_C|GetPlayerHudW _as_first_person_character))
  (bind _infotext (Variables|/Game/Blueprints/Widget/Player_Hud.Player_Hud_C|GetInfoText _playerhudw))
  (bind _infotext_2 (Variables|/Game/Blueprints/Widget/Player_Hud.Player_Hud_C|GetInfoText _playerhudw_2))
  (if (Variables|Default|GetisTraped)
    (Variables|/Game/FirstPersonBP/Blueprints/FirstPersonCharacter.FirstPersonCharacter_C|SetMouseInputUseable PlayerRef false)
    (Rendering|Components|TextRender|SetText _infotext_2 "Tuzak Sökülüyor")
    (Utilities|FlowControl|Delay 2.0)
    (Variables|/Game/FirstPersonBP/Blueprints/FirstPersonCharacter.FirstPersonCharacter_C|SetMouseInputUseable PlayerRef true)
    (Components|Activation|SetActive (Variables|/Script/Engine.Character|GetCharacterMovement _as_first_person_character) true false)
    (Rendering|Components|TextRender|SetText _infotext_2 "")
    (Actor|DestroyActor)
    (else
      (Variables|/Game/FirstPersonBP/Blueprints/FirstPersonCharacter.FirstPersonCharacter_C|SetMouseInputUseable PlayerRef false)
      (Components|Activation|SetActive _charactermovement false false)
      (Rendering|Components|TextRender|SetText _infotext "Tuzak Sökülüyor")
      (Utilities|FlowControl|Delay 2.0)
      (Variables|/Game/FirstPersonBP/Blueprints/FirstPersonCharacter.FirstPersonCharacter_C|SetMouseInputUseable PlayerRef true)
      (Components|Activation|SetActive _charactermovement true false)
      (Rendering|Components|TextRender|SetText _infotext "")
      (Actor|DestroyActor))))

(fn ConstructionScript)