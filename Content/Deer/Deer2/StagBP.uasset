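; StagBP is a stag actor that makes a one-way scripted walk along world X and then removes itself.
; While IsStagWalk is true, Tick plays the StagWalkTL timeline, which drives the root's absolute X position and keeps Y and Z.
; On finish it clears the flag and destroys the actor after a short delay.
; No live node here sets the flag; an older Timeline_0 chain that did is unconnected.
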(event EventBeginPlay)

(event Collision|EventActorBeginOverlap
  (params (OtherActor :type Actor%20Object%20Reference)))

(event EventTick
  (params (DeltaSeconds :type Float%20%28single-precision%29))
  (bind _defaultsceneroot (Variables|Default|GetDefaultSceneRoot))
  (bind _returnvalue (Transformation|GetWorldLocation _defaultsceneroot))
  (if (Variables|Default|GetisStagWalk)
    (bind _newtrack_0 (Timeline|StagWalkTL Play)
      (:Update
        (Transformation|SetWorldLocation _defaultsceneroot (Math|Vector|MakeVector _newtrack_0 (.y _returnvalue) (.z _returnvalue)) false false))
      (:Finished
        (Variables|Default|SetisStagWalk false)
        (Utilities|FlowControl|Delay 3.0)
        (Actor|DestroyActor)))))

(fn ConstructionScript)